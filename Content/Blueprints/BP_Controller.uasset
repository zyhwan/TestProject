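; BP_Controller lets the player paint on BP_Canvas actors using the Draw input axis.
; While the axis reads exactly 1.0, it line-traces on Visibility a short range forward from the player camera with complex collision.
; A hit canvas receives a Drawbrush call with the controller's brush texture and size, placed at the UV found from the hit through FindCollisionUV.
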(event `InputAxis|Draw`
  (params (AxisValue :type "Float (single-precision)"))
  (bind _returnvalue (`GameplayStatics.GetPlayerCameraManager` 0))
  (bind _returnvalue_2 (`self.K2_GetActorLocation` _returnvalue))
  (if (== AxisValue 1.0)
    (bind _outhit (`KismetSystemLibrary.LineTraceSingle` _returnvalue_2 (+ _returnvalue_2 (* (`self.GetActorForwardVector` _returnvalue) 1500.0)) "TraceTypeQuery1" true))
    (bind _asbp_canvas (cast `/Game/Blueprints/BP_Canvas` (`.HitActor` (`GameplayStatics.BreakHitResult` _outhit))))
    (`/Game/Blueprints/BP_Canvas.Drawbrush` _asbp_canvas (`self.Brush Texture`) (`self.Brush Size`) (`GameplayStatics.FindCollisionUV` _outhit))))

(fn `UserConstructionScript`)